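; Manager actor for the King of the Pill level that tracks how many pills remain and ends the level when none are left.
; BeginPlay sets the pill count, and the RemovePill event decrements it.
; At zero, it calls the exposure transition on the player's ThirdPersonCharacterOriginal, waits briefly, then loads the main menu level.
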(event `self.ReceiveBeginPlay`
  (set `self.PillsLeft` 16))

(event `RemovePill`
  (bind _pillsleft (`self.PillsLeft`))
  (`/Engine/EditorBlueprintResources/StandardMacros.DecrementInt` _pillsleft
    (:`  `
      (if (not (> _pillsleft 0))
        (bind _asthird_person_character_original (cast `/Game/ThirdPersonBP/Blueprints/ThirdPersonCharacterOriginal` (`GameplayStatics.GetPlayerCharacter` 0)))
        (`/Game/ThirdPersonBP/Blueprints/ThirdPersonCharacterOriginal.Exposure Transition Start` _asthird_person_character_original)
        (`KismetSystemLibrary.Delay` 2.0)
        (`GameplayStatics.OpenLevel` "MainMenu_LVL")))))

(fn `UserConstructionScript`)