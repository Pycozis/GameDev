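; Pill pickup Blueprint for King of the Pill that reacts when the player overlaps its Box trigger.
; On overlap by a ThirdPersonCharacterOriginal with a "Player"-tagged capsule, the Pill_Jump timeline moves the mesh by local Z offsets and smoke particles activate.
; It then calls RemovePill on the PillManager_Blueprint found in the level and destroys the Box, so the trigger cannot fire again.
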(event `self.Box.OnComponentBeginOverlap`
  (params (OverlappedComponent :type "PrimitiveComponent Object Reference") (OtherActor :type "Actor Object Reference") (OtherComp :type "PrimitiveComponent Object Reference") (OtherBodyIndex :type Integer) (bFromSweep :type Boolean) (SweepResult :type "HitResult Structure (by ref)"))
  (bind _asthird_person_character_original (cast `/Game/ThirdPersonBP/Blueprints/ThirdPersonCharacterOriginal` OtherActor))
  (if (`ActorComponent.ComponentHasTag` (`Character.CapsuleComponent` _asthird_person_character_original) "Player")
    (`|ExecutionSequence`
      (:`then_0`
        (bind (_direction _pillheight) (`Timeline|Pill_Jump` :!via `PlayFromStart`)
          (:`Update`
            (`SceneComponent.K2_AddLocalOffset` (`self.StaticMeshComponent`) (`KismetMathLibrary.MakeVector` 0.0 0.0 _pillheight) false false))))
      (:`then_1`
        (`ActorComponent.Activate` (`Emitter.ParticleSystemComponent` (`self.Smoke`)) false))
      (:`then_2`
        (bind _returnvalue (`GameplayStatics.GetActorOfClass` "/Game/Assignment/Josh/KingOfThePill/Blueprints/PillManager_Blueprint.PillManager_Blueprint_C"))
        (bind _aspill_manager_blueprint (cast `/Game/Assignment/Josh/KingOfThePill/Blueprints/PillManager_Blueprint` _returnvalue))
        (`/Game/Assignment/Josh/KingOfThePill/Blueprints/PillManager_Blueprint.RemovePill` _aspill_manager_blueprint))
      (:`then_3`
        (`ActorComponent.K2_DestroyComponent` (`self.Box`))))))

(fn `UserConstructionScript`)