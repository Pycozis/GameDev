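; A platform Blueprint that rises 1000 units when the player enters its Box trigger and moves back down when they leave.
; BeginPlay stores the root's world location as the starting point.
; Overlap events check for a ThirdPersonCharacter with a "Player"-tagged capsule, then play or reverse the Move_Platform timeline.
; The timeline's XValue drives an interpolation that sets the root's location without sweeping.
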(event `self.ReceiveBeginPlay`
  (set `self.Original Pos` (`SceneComponent.K2_GetComponentLocation` (`self.DefaultSceneRoot`))))

(event `self.Box.OnComponentBeginOverlap`
  (params (OverlappedComponent :type "PrimitiveComponent Object Reference") (OtherActor :type "Actor Object Reference") (OtherComp :type "PrimitiveComponent Object Reference") (OtherBodyIndex :type Integer) (bFromSweep :type Boolean) (SweepResult :type "HitResult Structure (by ref)"))
  (bind _asthird_person_character (cast `/Game/ThirdPersonBP/Blueprints/ThirdPersonCharacter` OtherActor))
  (if (`ActorComponent.ComponentHasTag` (`Character.CapsuleComponent` _asthird_person_character) "Player")
    (bind (_direction _x_value) (`Timeline|Move_Platform` :!label _label)
      (:`Update`
        (bind _returnvalue_location (`KismetMathLibrary.BreakTransform` (`KismetMathLibrary.TLerp` (`KismetMathLibrary.MakeTransform` (`self.Original Pos`)) (`KismetMathLibrary.MakeTransform` (+ (`self.Original Pos`) (0.0 0.0 1000.0))) _x_value)))
        (`SceneComponent.K2_SetWorldLocation` (`self.DefaultSceneRoot`) _returnvalue_location false false)))))

(event `self.Box.OnComponentEndOverlap`
  (params (OverlappedComponent :type "PrimitiveComponent Object Reference") (OtherActor :type "Actor Object Reference") (OtherComp :type "PrimitiveComponent Object Reference") (OtherBodyIndex :type Integer))
  (bind _asthird_person_character (cast `/Game/ThirdPersonBP/Blueprints/ThirdPersonCharacter` OtherActor))
  (if (`ActorComponent.ComponentHasTag` (`Character.CapsuleComponent` _asthird_person_character) "Player")
    (goto _label :!via `Reverse`)))

(fn `UserConstructionScript`)