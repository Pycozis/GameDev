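; Spotlight Blueprint whose shrinking light radius acts as a countdown to opening the "Half-Light" level.
; A timeline started on BeginPlay reduces the attenuation radius by a fixed step on every update, so the drain rate follows frame rate, and opens the level at a minimum radius.
; Tick watches an Expand flag, which nothing in this graph sets true, then enlarges the radius once and clears the flag.
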(event `self.ReceiveBeginPlay`
  (bind _spotlightcomponent (`self.SpotLightComponent`))
  (`Timeline|Timeline_0`
    (:`Update`
      (`LocalLightComponent.SetAttenuationRadius` _spotlightcomponent (- (`LocalLightComponent.AttenuationRadius` _spotlightcomponent) 0.25))
      (if (<= (`LocalLightComponent.AttenuationRadius` _spotlightcomponent) 200.0)
        (`GameplayStatics.OpenLevel` "Half-Light")))))

(event `self.ReceiveTick`
  (params (DeltaSeconds :type "Float (single-precision)"))
  (bind _spotlightcomponent (`self.SpotLightComponent`))
  (if (`self.Expand`)
    (`LocalLightComponent.SetAttenuationRadius` _spotlightcomponent (+ (`LocalLightComponent.AttenuationRadius` _spotlightcomponent) 50.0))
    (set `self.Expand` false)))

(fn `UserConstructionScript`)